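; BP_BossProjectile is a boss projectile that targets the player and damages combat characters it hits.
; On BeginPlay it sets the first player pawn's root component as the ProjectileMovement homing target.
; Hit applies damage only to BP_CombatCharacter actors and then destroys the projectile, ignoring anything else.
; Leftover disconnected nodes for an overlap check, alternate damage and homing never run.
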(event `self.ReceiveBeginPlay`
  (set `ProjectileMovementComponent.HomingTargetComponent` (`Actor.RootComponent` (`GameplayStatics.GetPlayerPawn` 0)) (`self.ProjectileMovement`)))

(event `self.ReceiveHit`
  (params (MyComp :type "PrimitiveComponent Object Reference") (Other :type "Actor Object Reference") (OtherComp :type "PrimitiveComponent Object Reference") (bSelfMoved :type Boolean) (HitLocation :type "Vector Structure") (HitNormal :type "Vector Structure") (NormalImpulse :type "Vector Structure") (Hit :type "HitResult Structure (by ref)"))
  (bind _asbp_combat_character (cast `/Game/Variant_Combat/Blueprints/BP_CombatCharacter` Other))
  (`GameplayStatics.ApplyDamage` _asbp_combat_character 0.5 null self)
  (`self.K2_DestroyActor`))

(fn `UserConstructionScript`)