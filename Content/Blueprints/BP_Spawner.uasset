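; BP_Spawner spawns the phase 1 boss, a BP_CombatEnemy1, and hands it its scene references.
; SpawnPhase1 waits out a fixed delay, then creates the enemy at the spawner's location with an enlarged scale.
; It then passes all TargetPoint actors as teleport points, plus the BP_CutsceneManager and BP_OverworldChange (as music manager) found through class lookups.
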(event `SpawnPhase1`
  (`KismetSystemLibrary.Delay` 14.0)
  (bind _returnvalue (`|SpawnActorFromClass` "/Game/Variant_Combat/Blueprints/AI/BP_CombatEnemy1.BP_CombatEnemy1_C" (`KismetMathLibrary.MakeTransform` (`self.K2_GetActorLocation`) (struct) (5.0 5.0 5.0)) "Undefined" "MultiplyWithRoot" null null))
  (bind _output_get (set `self.SpawnedBoss` _returnvalue))
  (bind _outactors (`GameplayStatics.GetAllActorsOfClass` "/Script/Engine.TargetPoint"))
  (`/Game/Variant_Combat/Blueprints/AI/BP_CombatEnemy1.SetTeleportPoints` _output_get _outactors)
  (bind _returnvalue_2 (`GameplayStatics.GetActorOfClass` "/Game/Blueprints/BP_CutsceneManager.BP_CutsceneManager_C"))
  (`/Game/Variant_Combat/Blueprints/AI/BP_CombatEnemy1.SetCutsceneManager` _output_get _returnvalue_2)
  (bind _returnvalue_3 (`GameplayStatics.GetActorOfClass` "/Game/Blueprints/BP_OverworldChange.BP_OverworldChange_C"))
  (`/Game/Variant_Combat/Blueprints/AI/BP_CombatEnemy1.SetMusicManager` _output_get _returnvalue_3))

(fn `UserConstructionScript`)